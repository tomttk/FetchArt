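; BP_RemoteImagePlane is an actor that shows a text label while the first-person character is near it.
; BeginPlay hides the TextComponent and applies its configured world size and render color.
; Box overlap events unhide the text when BP_FirstPersonCharacter enters and hide it again on exit.
; Despite the asset name, its graphs contain no image-loading logic.
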(event `self.ReceiveBeginPlay`
  (bind _textcomponent (`self.TextComponent`))
  ;[1 1 1] Hide an display/ Set text
  (`SceneComponent.SetHiddenInGame` _textcomponent true false)
  (`TextRenderComponent.SetWorldSize` _textcomponent (`self.SizeText`))
  (`TextRenderComponent.SetTextRenderColor` _textcomponent (`self.ColorValue`)))

(event `self.Box.OnComponentBeginOverlap`
  (params (OverlappedComponent :type "PrimitiveComponent Object Reference") (OtherActor :type "Actor Object Reference") (OtherComp :type "PrimitiveComponent Object Reference") (OtherBodyIndex :type Integer) (bFromSweep :type Boolean) (SweepResult :type "HitResult Structure (by ref)"))
  ;[1 1 1] Hide an display/ Set text
  (cast `/Game/Blueprints/BP_FirstPersonCharacter` OtherActor)
  (`SceneComponent.SetHiddenInGame` (`self.TextComponent`) false false))

(event `self.Box.OnComponentEndOverlap`
  (params (OverlappedComponent :type "PrimitiveComponent Object Reference") (OtherActor :type "Actor Object Reference") (OtherComp :type "PrimitiveComponent Object Reference") (OtherBodyIndex :type Integer))
  ;[1 1 1] Hide an display/ Set text
  (cast `/Game/Blueprints/BP_FirstPersonCharacter` OtherActor)
  (`SceneComponent.SetHiddenInGame` (`self.TextComponent`) true false))

(fn `UserConstructionScript`)